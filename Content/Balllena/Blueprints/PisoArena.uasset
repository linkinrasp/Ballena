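; PisoArena is a sand floor piece that places one randomly chosen whale on itself from its construction script.
; It gathers six arrow components' relative transforms, then randomly calls an orca (two variants), humpback or sperm whale function, with humpback weighted double.
; Each function adds a child actor component at a random one of those transforms.
; The event graph is inactive, and GetAttachPoint leaves the AttachPoint transform unconnected.
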(event EventBeginPlay)

(event Collision|EventActorBeginOverlap
  (params (OtherActor :type Actor%20Object%20Reference)))

(event EventTick
  (params (DeltaSeconds :type Float%20%28single-precision%29)))

(fn ConstructionScript
  (CallFunction|SetSpawnBallenas)
  (switch int (Math|Random|RandomIntegerinRange 0 4)
    (:0
      (CallFunction|SpawnOrca))
    (:1
      (CallFunction|SpawnOrca2))
    (:2
      (CallFunction|SpawnJorobada))
    (:3
      (CallFunction|SpawnCachalote))
    (:4
      (CallFunction|SpawnJorobada))))

(fn SetSpawnBallenas
  (Variables|Default|SetSpawnBallenas (Utilities|Array|MakeArray (Transformation|GetRelativeTransform (Variables|Default|GetArrow6)) (Transformation|GetRelativeTransform (Variables|Default|GetArrow5)) (Transformation|GetRelativeTransform (Variables|Default|GetArrow4)) (Transformation|GetRelativeTransform (Variables|Default|GetArrow3)) (Transformation|GetRelativeTransform (Variables|Default|GetArrow2)) (Transformation|GetRelativeTransform (Variables|Default|GetArrow1)))))

(fn SpawnOrca
  (bind _spawnballenas (Variables|Default|GetSpawnBallenas))
  (AddComponent|AddChildActorComponent false (Utilities|Array|Get(acopy) _spawnballenas (Math|Random|RandomIntegerinRange 0 (Utilities|Array|LastIndex _spawnballenas)))))

(fn SpawnOrca2
  (bind _spawnballenas (Variables|Default|GetSpawnBallenas))
  (AddComponent|AddChildActorComponent false (Utilities|Array|Get(acopy) _spawnballenas (Math|Random|RandomIntegerinRange 0 (Utilities|Array|LastIndex _spawnballenas)))))

(fn SpawnJorobada
  (bind _spawnballenas (Variables|Default|GetSpawnBallenas))
  (AddComponent|AddChildActorComponent false (Utilities|Array|Get(acopy) _spawnballenas (Math|Random|RandomIntegerinRange 0 (Utilities|Array|LastIndex _spawnballenas)))))

(fn SpawnCachalote
  (bind _spawnballenas (Variables|Default|GetSpawnBallenas))
  (AddComponent|AddChildActorComponent false (Utilities|Array|Get(acopy) _spawnballenas (Math|Random|RandomIntegerinRange 0 (Utilities|Array|LastIndex _spawnballenas)))))

(fn GetAttachPoint
  (return false))